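; BP_Enemy is an AI enemy that chases the player and offers horizontal and jump melee attacks.
; On BeginPlay it spawns a weapon onto its hand socket and starts AIMoveTo, which re-issues itself shortly after each successful arrival.
; Separately triggered attack events play montages and fire end dispatchers on completion or interruption.
; Only the horizontal attack first turns to face the player.
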(event Custom|WieldWeapon
  ;[0.15 0.15 0.15 0.5] Weapon
  (bind _returnvalue (Game|SpawnActorfromClass "/Game/YW/blueprint/BP_Weapon.BP_Weapon_C" (Transformation|GetActorTransform) "Undefined" "MultiplyWithRoot" 0 0))
  (Transformation|AttachComponentToComponent _returnvalue (Variables|Character|GetMesh) "Right_Weapon" "SnapToTarget" "SnapToTarget" "SnapToTarget" true)
  (Variables|Default|SetIsWieldingWeapon true))

(event Custom|ChasePlayer
  (AI|AIMoveTo self "0, 0, 0" (Game|GetPlayerCharacter 0) 1e+02 false
    (:OnSuccess
      (Utilities|FlowControl|Delay 0.2)
      (CallFunction|ChasePlayer))))

(event Custom|JampAttack
  ;[0.15 0.15 0.15 0.5] Jump Attack
  (Animation|Montage|PlayMontage (Variables|Character|GetMesh) "/Game/YW/Anims/Mon_JumpAttack.Mon_JumpAttack" 0.85
    (:OnCompleted
      _)
    (:OnInterrupted
      _))
  (Default|CallOnJumpAttackEnd))

(event Custom|Attack
  ;[0.15 0.15 0.15 0.5] Attack
  (Transformation|SetActorRotation (Math|Rotator|FindLookatRotation (Transformation|GetActorLocation) (Transformation|GetActorLocation (Game|Player|GetPlayerPawn 0))))
  (Animation|Montage|PlayMontage (Variables|Character|GetMesh) "/Game/YW/Anims/Mon_AttckHorizontal.Mon_AttckHorizontal"
    (:OnCompleted
      _)
    (:OnInterrupted
      _))
  (Default|CallOnAttackHorizonEnd))

(event EventBeginPlay
  (CallFunction|WieldWeapon)
  (CallFunction|ChasePlayer))

(fn ConstructionScript)