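; Knight boss enemy character with wake-up sequence, montage attacks, groggy state and two phases, exposing actions alongside AIC_Enemy's behavior tree.
; Overlap volumes drive the game mode's weapon-out UI, gated by saved data.
; Jump attack launches the knight along a projectile arc toward the player's predicted position.
; Tick displays HP, triggers phase two near half health with changed weapon damage, and on death stops AI and finishes the match.
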(event OnComponentBeginOverlap(UI_Within_Distance)
  (params (OverlappedComponent :type Primitive%20Component%20Object%20Reference) (OtherActor :type Actor%20Object%20Reference) (OtherComp :type Primitive%20Component%20Object%20Reference) (OtherBodyIndex :type Integer) (bFromSweep :type Boolean) (SweepResult :type Hit%20Result%20Structure%20%28by%20ref%29))
  ;[0.15 0.15 0.15 0.5] CollisionSetting
  (Utilities|Casting|CastToBP_Player OtherActor)
  (bind _asbp_game_instance (Utilities|Casting|CastToBP_GameInstance (Game|GetGameInstance)))
  (if (not (Variables|/Game/MW/Player/Blueprints/BP_SaveDeathCount.BP_SaveDeathCount_C|GetSaveDataWeaponOut (Variables|/Game/MW/Player/Blueprints/BP_GameInstance.BP_GameInstance_C|GetAs%20BP%20Save%20Death%20Count _asbp_game_instance)))
    (Default|DisplayWeaponOut (Variables|Default|GetMyGameMode))
    (Collision|SetCollisionEnabled (Variables|Default|GetUI_Within_Distance) "NoCollision")
    (Collision|SetCollisionEnabled (Variables|Default|GetUI_Within_Weapon_Distance) "QueryOnly")))

(event OnComponentBeginOverlap(UI_Within_Weapon_Distance)
  (params (OverlappedComponent :type Primitive%20Component%20Object%20Reference) (OtherActor :type Actor%20Object%20Reference) (OtherComp :type Primitive%20Component%20Object%20Reference) (OtherBodyIndex :type Integer) (bFromSweep :type Boolean) (SweepResult :type Hit%20Result%20Structure%20%28by%20ref%29))
  ;[0.15 0.15 0.15 0.5] CollisionSetting
  (Variables|/Game/MW/Player/Blueprints/BP_GameModeBase.BP_GameModeBase_C|SetWithin_WeaponOut_Distance (Variables|Default|GetMyGameMode) true))

(event OnComponentEndOverlap(UI_Within_Weapon_Distance)
  (params (OverlappedComponent :type Primitive%20Component%20Object%20Reference) (OtherActor :type Actor%20Object%20Reference) (OtherComp :type Primitive%20Component%20Object%20Reference) (OtherBodyIndex :type Integer))
  ;[0.15 0.15 0.15 0.5] CollisionSetting
  (Variables|/Game/MW/Player/Blueprints/BP_GameModeBase.BP_GameModeBase_C|SetWithin_WeaponOut_Distance (Variables|Default|GetMyGameMode) false))

(event Custom|LongRangeAttack
  (params (AttackTarget :type Actor%20Object%20Reference))
  ;[0.15 0.15 0.15 0.5] JumpAttack
  (Variables|Default|SetAttackType 1)
  (CallFunction|LookPlayer)
  (bind _notifyname (Animation|Montage|PlayMontage (Variables|Character|GetMesh) "/Game/YW/Aim_Montage/Enemy_Montage_Jump.Enemy_Montage_Jump")
    (:OnCompleted
      (Default|CallOnJumpAttackEnd :!label _label))
    (:OnInterrupted
      (goto _label))
    (:OnNotifyBegin
      (Development|PrintString "Norify")
      (switch name _notifyname
        (:Jump
          (CallFunction|JumptoTarget AttackTarget))
        (:Slash
          (CallFunction|Slash))))))

(event Custom|Slash
  (bind _returnvalue (Transformation|GetActorLocation))
  ;[0.15 0.15 0.15 0.5] JumpAttack
  (bind _returnvalue_2 (Collision|MultiSphereTraceForObjects _returnvalue (+ _returnvalue (* (Transformation|GetActorForwardVector) 2e+02)) 2e+01 (Variables|Default|GetObject%20Types) false 0 "None"))
  (Development|PrintString (Utilities|String|ToString(Boolean) _returnvalue_2)))

(event Custom|CustomEvent)

(event Custom|ChasePlayer
  (params (Distance :type Float%20%28double-precision%29))
  ;[0.15 0.15 0.15 0.5] ChasePlayer
  (CallFunction|SetMaxWalkSpeed "NewEnumerator3")
  (AI|AIMoveTo self "0, 0, 0" (Game|GetPlayerCharacter 0) Distance false
    (:OnSuccess
      (Utilities|FlowControl|Delay 2.0))))

(event Custom|WieldWeapon
  ;[0.15 0.15 0.15 0.5] Weapon
  (bind _returnvalue (Game|SpawnActorfromClass "/Game/YW/blueprint/BP_Weapon.BP_Weapon_C" (Transformation|GetActorTransform) "Undefined" "MultiplyWithRoot" 0 0))
  (Transformation|AttachComponentToComponent _returnvalue (Variables|Character|GetMesh) "Right_Weapon" "SnapToTarget" "SnapToTarget" "SnapToTarget" true)
  (Variables|Default|SetIsWieldingWeapon true))

(event Custom|JumpToTarget
  (params (AttackTarget :type Actor%20Object%20Reference))
  ;[0.15 0.15 0.15 0.5] JumpAttack
  (bind _location (CallFunction|CalculateFutureActorLocation AttackTarget 1.0))
  (bind _outlaunchvelocity (Game|SuggestProjectileVelocityCustomArc (Transformation|GetActorLocation) (Math|Vector|MakeVector (.x _location) (.y _location) (+ (.z _location) 5e+01)) 0.0 0.7))
  (Variables|Default|SetTest _outlaunchvelocity)
  (Character|LaunchCharacter (Math|Vector|MakeVector (* (.x (Variables|Default|GetTest)) 1.7) (* (.y (Variables|Default|GetTest)) 1.7) (.z (Variables|Default|GetTest))) true true))

(event Custom|EnemyWakeUp
  ;[0.15 0.15 0.15 0.5] Wake Up Motion
  (Collision|SetCollisionEnabled (Variables|Default|GetUI_Within_Weapon_Distance) "NoCollision")
  (Utilities|FlowControl|Delay 7.0)
  (Animation|Montage|PlayMontage (Variables|Character|GetMesh) "/Game/YW/Aim_Montage/Enemy_Pickup_Wakeup.Enemy_Pickup_Wakeup"
    (:then
      (Utilities|FlowControl|Delay 0.2)
      (bind _asabp_knight (Utilities|Casting|CastToABP_Knight (Components|SkeletalMesh|GetAnimInstance (Variables|Character|GetMesh))))
      (Variables|/Game/YW/blueprint/ABP_Knight.ABP_Knight_C|SetABP_WeaponOut _asabp_knight true)
      (Variables|Default|SetIsWeaponOut true)
      (Utilities|FlowControl|Delay 3.0)
      (Default|ManageBGM (Variables|Default|GetMyGameMode)))
    (:OnCompleted
      (Default|CallOnAwakeEnd :!label _label))
    (:OnInterrupted
      (goto _label))))

(event EventBeginPlay
  (Variables|Default|SetDeadFlag false)
  (bind _asbp_game_mode_base (Utilities|Casting|CastToBP_GameModeBase (Game|GetGameMode)))
  (Variables|Default|SetMyGameMode _asbp_game_mode_base)
  ;[0.15 0.15 0.15 0.5] Initial Setting
  (Collision|SetCollisionEnabled (Variables|Default|GetUI_Within_Weapon_Distance) "NoCollision")
  (Variables|Default|SetHP (Variables|Default|GetMaxHP))
  (Variables|Default|SetIsDead false)
  (Variables|Default|SetIsWeaponOut false)
  ;[0.15 0.15 0.15 0.5] UI 띄우는 창 Collision setting
  (bind _asbp_game_instance (Utilities|Casting|CastToBP_GameInstance (Game|GetGameInstance)))
  (if (Variables|/Game/MW/Player/Blueprints/BP_SaveDeathCount.BP_SaveDeathCount_C|GetSaveDataWeaponOut (Variables|/Game/MW/Player/Blueprints/BP_GameInstance.BP_GameInstance_C|GetAs%20BP%20Save%20Death%20Count _asbp_game_instance))
    (Collision|SetCollisionEnabled (Variables|Default|GetUI_Within_Distance) "NoCollision")
    (else
      (Collision|SetCollisionEnabled (Variables|Default|GetUI_Within_Distance) "QueryOnly"))))

(event EventTick
  (params (DeltaSeconds :type Float%20%28single-precision%29))
  (bind _returnvalue (Transformation|GetActorLocation))
  (bind _mygamemode (Variables|Default|GetMyGameMode))
  (bind _charactermovement (Variables|Character|GetCharacterMovement))
  (bind _mesh (Variables|Character|GetMesh))
  (bind _returnvalue_2 (Transformation|GetWorldLocation _mesh))
  ;[0.15 0.15 0.15 0.5] HP text render
  (Rendering|Components|TextRender|SetText (Variables|Default|GetTextRender) (Utilities|Text|ToText(Integer) (Variables|Default|GetHP)))
  ;[0.15 0.15 0.15 0.5] Is 2phase?
  (if (and (<= (/ (Math|Conversions|ToFloat(Integer) (Variables|Default|GetHP)) (Math|Conversions|ToFloat(Integer) (Variables|Default|GetMaxHP))) 0.55) (== (Variables|Default|GetPhaseFlag) false))
    (bind _returnvalue_3 (Actor|GetActorOfClass "/Game/YW/blueprint/BP_Weapon.BP_Weapon_C"))
    (Variables|/Game/YW/blueprint/BP_Weapon.BP_Weapon_C|SetEnemy_Damage _returnvalue_3 40)
    (Variables|Default|SetIsPhase2 true)
    (Variables|Default|SetPhaseFlag true)
    (Animation|Montage|PlayMontage (Variables|Character|GetMesh) "/Game/YW/Aim_Montage/Enemy_Phase2.Enemy_Phase2"
      (:then
        _)
      (:OnCompleted
        _))
    (Utilities|FlowControl|Delay 2.0)
    (else
      ;[0.15 0.15 0.15 0.5] IsDead?
      (if (and (<= (Variables|Default|GetHP) 0) (== (Variables|Default|GetDeadFlag) false))
        (Variables|Default|SetDeadFlag true)
        (Components|Movement|StopMovementImmediately _charactermovement)
        (Pawn|Components|CharacterMovement|DisableMovement _charactermovement)
        (bind _asaic_enemy (Utilities|Casting|CastToAIC_Enemy (Pawn|GetController)))
        (Default|KillBT _asaic_enemy)
        (Variables|Default|SetIsDead true)
        (Variables|/Game/MW/Player/Blueprints/BP_GameModeBase.BP_GameModeBase_C|SetPlayerLose _mygamemode 0)
        (Default|WhenFinished _mygamemode)
        (Utilities|FlowControl|Delay 3.5)
        (Effects|SpawnEmitteratLocation "/Game/YW/VFX/P_Sparks_B.P_Sparks_B" _returnvalue_2)
        (Effects|SpawnEmitteratLocation "/Game/YW/VFX/P_Smoke_B.P_Smoke_B" _returnvalue_2 "0, 0, 0" "10.000000,10.000000,10.000000")
        (Utilities|FlowControl|Delay 3.5)
        (Default|RemoveFinishUI (Variables|Default|GetMyGameMode))
        (Collision|SetCollisionEnabled (Variables|Collision|GetCapsuleComponent) "NoCollision")
        (Collision|SetCollisionEnabled (Variables|Character|GetMesh) "NoCollision")
        (Transformation|SetActorLocation (Math|Vector|MakeVector (.x _returnvalue) (.y _returnvalue) -2e+01) false false)))))

(event EventGroggy
  ;[0.15 0.15 0.15 0.5] 그로기
  (Variables|Default|SetIsGroggying true)
  (Animation|PlayAnimMontage "/Game/YW/Aim_Montage/Enemy_Groggy_Montage.Enemy_Groggy_Montage" 1.0 "None")
  (Utilities|FlowControl|Delay 7.0)
  (Variables|Default|SetIsGroggying false))

(event EventJampAttack)

(fn ConstructionScript)

(fn LookPlayer
  (bind _returnvalue (Transformation|GetActorLocation))
  (bind _returnvalue_2 (Game|Player|GetPlayerPawn 0))
  (bind _returnvalue_3 (Transformation|GetActorLocation _returnvalue_2))
  (bind _returnvalue_4 (Math|Rotator|FindLookatRotation _returnvalue _returnvalue_3))
  (Transformation|SetActorRotation (Math|Rotator|MakeRotator (.roll _returnvalue_4) 0.0 (.yaw _returnvalue_4))))

(fn CalculateFutureActorLocation
  (params (Actor :type Actor%20Object%20Reference) (Time :type Float%20%28double-precision%29))
  (return (+ (Transformation|GetActorLocation Actor) (* (* (Transformation|GetVelocity Actor) "1.000000,1.000000,0.000000") Time))))

(fn AttackDown
  (Variables|Default|SetAttackType 1)
  (CallFunction|LookPlayer)
  (bind _returnvalue (Animation|PlayAnimMontage "/Game/YW/Aim_Montage/AI_Enemy_Attack_Montage.AI_Enemy_Attack_Montage" 1.0 "Attack3"))
  (return _returnvalue))

(fn AttackFront
  (Variables|Default|SetAttackType 0)
  (CallFunction|LookPlayer)
  (bind _returnvalue (Animation|PlayAnimMontage "/Game/YW/Aim_Montage/AI_Enemy_Attack_Montage.AI_Enemy_Attack_Montage" 1.0 "Attack2"))
  (return _returnvalue))

(fn AttackHorizonal
  (Variables|Default|SetAttackType 1)
  (CallFunction|LookPlayer)
  (bind _returnvalue (Animation|PlayAnimMontage "/Game/YW/Aim_Montage/AI_Enemy_Attack_Montage.AI_Enemy_Attack_Montage" 1.0 "Attack1"))
  (return _returnvalue))

(fn AttackUp
  (Variables|Default|SetAttackType 0)
  (CallFunction|LookPlayer)
  (Animation|PlayAnimMontage "/Game/YW/Aim_Montage/AI_Enemy_Attack_Montage.AI_Enemy_Attack_Montage" 1.0 "AttackUp")
  (return 0.0))

(fn Awake)

(fn Die
  (Development|PrintString "Die")
  (bind _returnvalue (Animation|PlayAnimMontage "/Game/YW/Aim_Montage/Enemy_Dead_Montage.Enemy_Dead_Montage" 1.0 "Death"))
  (return _returnvalue))

(fn SetMaxWalkSpeed
  (params (Speed :type E_MovementSpeed%20Enum :default "NewEnumerator0"))
  (bind _output_get (Variables|/Script/Engine.CharacterMovementComponent|SetMaxWalkSpeed (Variables|Character|GetCharacterMovement) (Utilities|Select :Index Speed :NewEnumerator0 0.0 :NewEnumerator1 2.5e+02 :NewEnumerator2 4e+02 :NewEnumerator3 1e+03)))
  (return _output_get))