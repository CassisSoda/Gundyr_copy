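; BP_Weapon is an enemy lance weapon that detects hits on the player and applies their effects.
; Attack start and done events toggle the lance collision, and overlapping the player sets an IsHit flag.
; Enemy_Hit_Check passes that flag to WhenPlayerHit, then clears it.
; WhenPlayerHit triggers the player's HitEvent, then drains stamina when guarding or subtracts EnemyDamage from Hp unless rolling.
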(event OnComponentBeginOverlap(LanceCollision)
  (params (OverlappedComponent :type Primitive%20Component%20Object%20Reference) (OtherActor :type Actor%20Object%20Reference) (OtherComp :type Primitive%20Component%20Object%20Reference) (OtherBodyIndex :type Integer) (bFromSweep :type Boolean) (SweepResult :type Hit%20Result%20Structure%20%28by%20ref%29))
  ;[0.15 0.15 0.15 0.5] Collsion 처리
  (bind _asbp_player (Utilities|Casting|CastToBP_Player (Game|Player|GetPlayerPawn 0)))
  (if (== _asbp_player OtherActor)
    (Variables|Default|SetIsHit true)))

(event OnComponentEndOverlap(LanceCollision)
  (params (OverlappedComponent :type Primitive%20Component%20Object%20Reference) (OtherActor :type Actor%20Object%20Reference) (OtherComp :type Primitive%20Component%20Object%20Reference) (OtherBodyIndex :type Integer))
  ;[0.15 0.15 0.15 0.5] Collsion 처리
  (CallFunction|EnemyAttackDone))

(event Custom|Enemy_Attack_Done
  ;[0.15 0.15 0.15 0.5] 창을 휘두를 때만 충돌
  (Collision|SetCollisionEnabled (Variables|Default|GetLance%20Collision) "NoCollision"))

(event Custom|Enemy_Attack_Start
  ;[0.15 0.15 0.15 0.5] 창을 휘두를 때만 충돌
  (Collision|SetCollisionEnabled (Variables|Default|GetLance%20Collision) "QueryAndPhysics"))

(event Custom|Enemy_Hit_Check
  ;[0.15 0.15 0.15 0.5] 피격판정
  (CallFunction|WhenPlayerHit (Variables|Default|GetIsHit))
  (Variables|Default|SetIsHit false))

(event EventBeginPlay)

(event Collision|EventActorBeginOverlap
  (params (OtherActor :type Actor%20Object%20Reference)))

(event EventTick
  (params (DeltaSeconds :type Float%20%28single-precision%29)))

(fn ConstructionScript)

(fn WhenPlayerHit
  (params (isHit :type Boolean))
  (if isHit
    (bind _asbp_player (Utilities|Casting|CastToBP_Player (Game|Player|GetPlayerPawn 0)))
    (Default|HitEvent _asbp_player (Variables|Default|GetIsHit) (Transformation|GetActorLocation))
    (if (Variables|/Game/MW/Player/Blueprints/BP_Player.BP_Player_C|GetIsGuarding _asbp_player)
      ;[0.15 0.15 0.15 0.5] 가드중이라면 스테미나 감소
      (bind _output_get (Variables|/Game/MW/Player/Blueprints/BP_Player.BP_Player_C|SetStamina _asbp_player (- (Variables|/Game/MW/Player/Blueprints/BP_Player.BP_Player_C|GetStamina _asbp_player) 6e+01)))
      (if (<= _output_get 0.0)
        (Variables|/Game/MW/Player/Blueprints/BP_Player.BP_Player_C|SetStamina _asbp_player 0.0))
      (else
        ;[0.15 0.15 0.15 0.5] 구르는 중이 아니면 체력 감소
        (if (not (Variables|/Game/MW/Player/Blueprints/BP_Player.BP_Player_C|GetIsRolling _asbp_player))
          (Variables|/Game/MW/Player/Blueprints/BP_Player.BP_Player_C|SetHp _asbp_player (- (Variables|/Game/MW/Player/Blueprints/BP_Player.BP_Player_C|GetHp _asbp_player) (Variables|Default|GetEnemy_Damage))))))))