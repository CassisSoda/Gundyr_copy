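; Interactable Spiral Sword actor that attaches to the player when taken and removes itself afterwards.
; On BeginPlay it destroys itself if the death-count save held by the game instance already has SaveDataWeaponOut set.
; Interaction start snaps it to the player mesh's SpiralSocket, then after a short delay spawns a blood burst just below the BP_Knight actor's location.
; Interaction end destroys the actor.
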(event Custom|Interaction_Start
  (bind _asbp_player (Utilities|Casting|CastToBP_Player (Game|Player|GetPlayerPawn 0)))
  (Transformation|AttachComponentToComponent (Variables|/Script/Engine.Character|GetMesh _asbp_player) "SpiralSocket" "SnapToTarget" "SnapToTarget" "SnapToTarget" true)
  (bind _returnvalue (Actor|GetActorOfClass "/Game/YW/blueprint/BP_Knight.BP_Knight_C"))
  (Utilities|FlowControl|Delay 0.7)
  (Effects|SpawnEmitteratLocation "/Game/YW/VFX/P_Blood_Burst.P_Blood_Burst" (Math|Vector|MakeVector (.x (Transformation|GetActorLocation _returnvalue)) (.y (Transformation|GetActorLocation _returnvalue)) (- (.z (Transformation|GetActorLocation _returnvalue)) 7e+01)) "90.000000,0.000000,0.000000"))

(event Custom|Interaction_End
  (Actor|DestroyActor))

(event EventBeginPlay
  (bind _asbp_game_instance (Utilities|Casting|CastToBP_GameInstance (Game|GetGameInstance)))
  (if (Variables|/Game/MW/Player/Blueprints/BP_SaveDeathCount.BP_SaveDeathCount_C|GetSaveDataWeaponOut (Variables|/Game/MW/Player/Blueprints/BP_GameInstance.BP_GameInstance_C|GetAs%20BP%20Save%20Death%20Count _asbp_game_instance))
    (Actor|DestroyActor)))

(event Collision|EventActorBeginOverlap
  (params (OtherActor :type Actor%20Object%20Reference)))

(event EventTick
  (params (DeltaSeconds :type Float%20%28single-precision%29)))

(fn ConstructionScript)