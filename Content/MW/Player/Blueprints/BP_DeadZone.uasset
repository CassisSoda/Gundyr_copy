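; BP_DeadZone is a kill zone actor that triggers the player's death when BP_Player overlaps it.
; On overlap, it plays the death montage at half speed and checks whether the level's BP_Knight is already dead.
; If the knight is dead, it calls YouDeadAfterWin on the game mode and AfterEnemyDead on the player; otherwise it calls the player's IsDead.
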(event EventBeginPlay)

(event Collision|EventActorBeginOverlap
  (params (OtherActor :type Actor%20Object%20Reference))
  (bind _asbp_player (Utilities|Casting|CastToBP_Player OtherActor))
  (bind _returnvalue (Actor|GetActorOfClass "/Game/YW/blueprint/BP_Knight.BP_Knight_C"))
  (Animation|Montage|PlayMontage (Variables|/Script/Engine.Character|GetMesh _asbp_player) "/Game/MW/Player/Animation/Montage/Player_Death_Montage.Player_Death_Montage" 0.5 0.0 "Death1"
    (:then
      (if (Variables|/Game/YW/blueprint/BP_Knight.BP_Knight_C|GetIsDead _returnvalue)
        (bind _asbp_game_mode_base (Utilities|Casting|CastToBP_GameModeBase (Game|GetGameMode)))
        (Default|YouDeadAfterWin _asbp_game_mode_base)
        (Default|AfterEnemyDead _asbp_player)
        (else
          (Default|IsDead _asbp_player))))))

(event EventTick
  (params (DeltaSeconds :type Float%20%28single-precision%29)))

(fn ConstructionScript)