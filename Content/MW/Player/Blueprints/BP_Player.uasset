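; Player character for melee combat with sword combos, guard, parry, potion healing and directional hit or death reactions.
; Enhanced Input drives the actions, with one key splitting into dash or roll by hold time and lock-on rolls following movement direction.
; Montages play the actions, while events toggle sword and parry collision windows.
; Actions spend or gate stamina; Tick updates its drain and regeneration, interpolated speed, gradual healing and text readouts.
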(event OnComponentBeginOverlap(SwordCollision)
  (params (OverlappedComponent :type Primitive%20Component%20Object%20Reference) (OtherActor :type Actor%20Object%20Reference) (OtherComp :type Primitive%20Component%20Object%20Reference) (OtherBodyIndex :type Integer) (bFromSweep :type Boolean) (SweepResult :type Hit%20Result%20Structure%20%28by%20ref%29))
  ;[0.15 0.15 0.15 0.5] Sword - Enemy 충돌처리
  (bind _asbp_knight (Utilities|Casting|CastToBP_Knight OtherActor))
  (if (not (Variables|Default|GetIsHit))
    (Variables|/Game/YW/blueprint/BP_Knight.BP_Knight_C|SetHP _asbp_knight (- (Variables|/Game/YW/blueprint/BP_Knight.BP_Knight_C|GetHP _asbp_knight) (Variables|Default|GetPlayerDamage)))))

(event OnComponentEndOverlap(SwordCollision)
  (params (OverlappedComponent :type Primitive%20Component%20Object%20Reference) (OtherActor :type Actor%20Object%20Reference) (OtherComp :type Primitive%20Component%20Object%20Reference) (OtherBodyIndex :type Integer))
  ;[0.15 0.15 0.15 0.5] Sword - Enemy 충돌처리
  (CallFunction|AttackDone))

(event Custom|DrinkPotion
  ;[0.15 0.15 0.15 0.5] 애니메이션 재생 시 손에 포션 스폰 /  체력 처리
  (bind _returnvalue (Game|SpawnActorfromClass "/Game/MW/Player/Blueprints/BP_Potion.BP_Potion_C" (Transformation|GetWorldTransform (Variables|Default|GetPotionPosition)) "Undefined" "MultiplyWithRoot" 0 0))
  (Transformation|AttachComponentToComponent _returnvalue (Variables|Character|GetMesh) "Potion" "SnapToTarget" "SnapToTarget" "SnapToTarget" true))

(event Custom|CheckNextCombo
  (bind _mesh (Variables|Character|GetMesh))
  ;[0.15 0.15 0.15 0.5] Attack
  (if (Variables|Default|GetIsChainAttacking)
    (if (> (Variables|Default|GetStamina) 0.0)
      (Variables|Default|SetIsChainAttacking false)
      (switch int (Variables|Default|GetComboCount) ; 콤보에 따른 분기
        (:0
          (Variables|Default|SetPlayerDamage 50)
          (Animation|Montage|PlayMontage _mesh "/Game/MW/Player/Animation/Montage/Attack_Montage.Attack_Montage" 1.0 0.0 "attack1" false
            (:then
              (Variables|Default|SetComboCount 1)
              (bind _output_get (Variables|Default|SetStamina (- (Variables|Default|GetStamina) 3e+01) :!label _label))
              (if (<= _output_get 0.0)
                (Variables|Default|SetStamina 0.0)))
            (:OnInterrupted
              (Variables|Default|SetIsAttacking false :!label _label_2))))
        (:1
          (Variables|Default|SetPlayerDamage 50)
          (Animation|Montage|PlayMontage _mesh "/Game/MW/Player/Animation/Montage/Attack_Montage.Attack_Montage" 1.0 0.0 "attack2" false
            (:then
              (Variables|Default|SetComboCount 0)
              (goto _label))
            (:OnInterrupted
              (goto _label_2))))))))

(event Custom|ParryDone
  ;[0.15 0.15 0.15 0.5] 모션중에만 패리 콜리전 ON
  (Collision|SetCollisionEnabled (Variables|Default|GetParry%20Collision) "NoCollision")
  (Variables|Default|SetGuardType -1))

(event Custom|ParryEnd
  (Variables|Default|SetIsParrying false)
  (Variables|Default|SetRecoveryingStamina 6e+01)
  (Utilities|FlowControl|Delay 0.5)
  (Variables|Default|SetStaminaRecovery 1))

(event Custom|Anim_AttEnd
  ;[0.15 0.15 0.15 0.5] Attack
  ;;[0.15 0.15 0.15 0.5] 공격 끝날 때
  (Utilities|FlowControl|Sequence
    (:then_0
      (Variables|Default|SetIsAttacking false)
      (Variables|Default|SetIsChainAttacking false)
      (Variables|Default|SetComboCount 0))
    (:then_1
      (Variables|Default|SetRecoveryingStamina 4e+01)
      (Utilities|FlowControl|Delay 0.5)
      (Variables|Default|SetStaminaRecovery 1))))

(event Custom|AttackDone
  ;[0.15 0.15 0.15 0.5] 칼을 휘두를 때만 충돌
  (Collision|SetCollisionEnabled (Variables|Default|GetSword%20Collision) "NoCollision"))

(event Custom|AttackStart
  ;[0.15 0.15 0.15 0.5] 칼을 휘두를 때만 충돌
  (Collision|SetCollisionEnabled (Variables|Default|GetSword%20Collision) "QueryAndPhysics"))

(event Custom|Hit_Event
  (params (IsHit :type Boolean) (Direction :type Vector) (AttType :type Integer))
  (bind _returnvalue (Transformation|GetActorLocation))
  (bind _mesh (Variables|Character|GetMesh))
  (bind _returnvalue_2 (- Direction _returnvalue))
  ;[0.15 0.15 0.15 0.5] 피격 / 맞은 방향애 따른 몽타주 출력
  (Variables|Default|SetIsHit IsHit)
  (Variables|Default|SetAtt%20Type AttType)
  (if (or (Variables|Default|GetIsRolling) (Variables|Default|GetIsParrying))
    (Variables|Default|SetIsHit false)
    (else
      (bind _output_get (Variables|Default|SetDamagingPosition (Math|Vector|Normalize (Math|Transform|InverseTransformDirection (Transformation|GetActorTransform) _returnvalue_2))))
      (bind _returnvalue_3 (Actor|GetActorOfClass "/Game/YW/blueprint/BP_Weapon.BP_Weapon_C"))
      (if (< (Variables|/Game/YW/blueprint/BP_Weapon.BP_Weapon_C|GetEnemy_Damage _returnvalue_3) (Variables|Default|GetHp))
        (if (Variables|Default|GetIsGuarding)
          (Animation|Montage|PlayMontage _mesh "/Game/MW/Player/Animation/Montage/Hit_Montage.Hit_Montage" 1.0 0.0 "Hit_Shield"
            (:then
              (CallFunction|CancelStatus :!label _label)))
          (elif (== (Variables|Default|GetAtt%20Type) 1)
            (Transformation|SetActorRotation (Math|Rotator|MakeRotator 0.0 0.0 (.Yaw (Math|Rotator|BreakRotator (Math|Conversions|RotationFromXVector (Math|Vector|Normalize _returnvalue_2))))) true)
            (Collision|SetCollisionEnabled (Variables|Collision|GetCapsuleComponent) "NoCollision")
            (Animation|Montage|PlayMontage _mesh "/Game/MW/Player/Animation/Montage/Hit_Airborne_Montage.Hit_Airborne_Montage"
              (:then
                (goto _label)))
            (else
              (if (> (.X (Math|Vector|BreakVector _output_get)) 0.4)
                (Animation|Montage|PlayMontage _mesh "/Game/MW/Player/Animation/Montage/Hit_Montage.Hit_Montage" 1.0 0.0 "Hit_R"
                  (:then
                    _))
                (elif (< (.X (Math|Vector|BreakVector _output_get)) -0.4)
                  (Animation|Montage|PlayMontage _mesh "/Game/MW/Player/Animation/Montage/Hit_Montage.Hit_Montage" 1.0 0.0 "Hit_L"
                    (:then
                      _))
                  (else
                    (Animation|Montage|PlayMontage _mesh "/Game/MW/Player/Animation/Montage/Hit_Montage.Hit_Montage" 1.0 0.0 "Hit_F"
                      (:then
                        _)))))
              (CallFunction|CancelStatus))))
        (else
          (CallFunction|DeathCheck (Variables|Default|GetAtt%20Type)))))))

(event Custom|OnCharacterCollision
  (Collision|SetCollisionEnabled (Variables|Collision|GetCapsuleComponent) "QueryAndPhysics"))

(event Custom|DeathCheck
  (params (Type :type Integer))
  (bind _mesh (Variables|Character|GetMesh))
  (bind _capsulecomponent (Variables|Collision|GetCapsuleComponent))
  ;[0.15 0.15 0.15 0.5] 사망 체크
  (switch int Type
    (:0
      (Animation|Montage|PlayMontage _mesh "/Game/MW/Player/Animation/Montage/Player_Death_Montage.Player_Death_Montage" 1.0 0.0 "Death_0"
        (:then
          (Collision|SetCollisionEnabled _capsulecomponent "NoCollision"))))
    (:1
      (Animation|Montage|PlayMontage _mesh "/Game/MW/Player/Animation/Montage/Player_Death_Montage.Player_Death_Montage" 1.0 0.0 "Death_1"
        (:then
          (Collision|SetCollisionEnabled _capsulecomponent "NoCollision"))))))

(event Custom|ParryUpdate
  (Rendering|Components|TextRender|SetText (Variables|Default|GetParry) (Utilities|Text|ToText(String) (Variables|Default|GetSuccess))))

(event Custom|ParryStart
  ;[0.15 0.15 0.15 0.5] 모션중에만 패리 콜리전 ON
  (Collision|SetCollisionEnabled (Variables|Default|GetParry%20Collision) "QueryOnly"))

(event Input|EnhancedActionEvents|EnhancedInputActionIA_Dash_And_Roll
  (params (ActionValue :type Boolean) (ElapsedSeconds :type Float%20%28double-precision%29) (TriggeredSeconds :type Float%20%28double-precision%29) (InputAction :type Input%20Action%20Object%20Reference :default "/Game/MW/Player/Inputs/IA_Dash_And_Roll.IA_Dash_And_Roll"))
  (bind _mesh (Variables|Character|GetMesh))
  (:Triggered
    ;[0.15 0.15 0.15 0.5] 스페이스바 입력 시간에 따른 분기 - Dash / Roll
    (Variables|Default|SetPressingTime (+ (Variables|Default|GetPressingTime) (Utilities|Time|GetWorldDeltaSeconds)))
    ;[0.15 0.15 0.15 0.5] Walk / Dash switch
    (if (>= (Variables|Default|GetPressingTime) (Variables|Default|GetRollLimitTime))
      (if (> (Variables|Default|GetStamina) 0.0)
        (Variables|Default|SetIsRunning true)
        (Variables|Default|SetDrowningStamina 5e+01)
        (Variables|Default|SetStaminaRecovery -1)
        (else
          (Utilities|FlowControl|Sequence :!label _label
            (:then_0
              (Variables|Default|SetIsRunning false)
              (Variables|Default|SetPressingTime 0.0))
            (:then_1
              (Variables|Default|SetRecoveryingStamina 6e+01)
              (Variables|Default|SetStaminaRecovery 0)
              (Utilities|FlowControl|Delay 1.0)
              (Variables|Default|SetStaminaRecovery 1)))))))
  (:Started
    (Variables|Default|SetStaminaRecovery 0))
  (:Completed
    (if (< (Variables|Default|GetPressingTime) (Variables|Default|GetRollLimitTime))
      ;[0.15 0.15 0.15 0.5] Rolling ( When is Not rolling)
      (if (Math|Boolean|ANDBoolean (> (Variables|Default|GetStamina) 0.0) (not (Variables|Default|GetIsRolling)) (not (Variables|Default|GetIsRunning)) (not (Variables|Default|GetIsAttacking)) (not (Variables|Default|GetIsHit)) (not (Variables|Default|GetIsParrying)))
        (Utilities|FlowControl|Sequence
          (:then_0
            (Variables|Default|SetStaminaRecovery 0)
            (Variables|Default|SetRecoveryingStamina 4e+01)
            (Variables|Default|SetPressingTime 0.0))
          (:then_1
            (Variables|Default|SetIsRolling true)
            (bind _output_get (Variables|Default|SetStamina (Math|Conversions|ToFloat(Integer) (- (Variables|Default|GetStamina) 35))))
            (if (<= _output_get 0.0)
              (Variables|Default|SetStamina 0.0)))
          (:then_2
            (if (not (Variables|Default|GetIsLockOn))
              (Animation|Montage|PlayMontage (Variables|Character|GetMesh) "/Game/MW/Player/Animation/Montage/Roll_Montage.Roll_Montage" 1.0 0.0 "Roll_F"
                (:then
                  (CallFunction|CancelStatus)))
              (else
                (bind _asabp_player (Utilities|Casting|CastToABP_Player (Components|SkeletalMesh|GetAnimInstance (Variables|Character|GetMesh))))
                (if (and (>= (Variables|/Game/MW/Player/Blueprints/ABP_Player.ABP_Player_C|GetDirection _asabp_player) -1.8e+02) (< (Variables|/Game/MW/Player/Blueprints/ABP_Player.ABP_Player_C|GetDirection _asabp_player) -135.0))
                  (Animation|Montage|PlayMontage _mesh "/Game/MW/Player/Animation/Montage/Roll_Montage.Roll_Montage" 1.0 0.0 "Roll_BL"
                    (:then
                      (CallFunction|CancelStatus :!label _label_2)))
                  (elif (and (> (Variables|/Game/MW/Player/Blueprints/ABP_Player.ABP_Player_C|GetDirection _asabp_player) 135.0) (<= (Variables|/Game/MW/Player/Blueprints/ABP_Player.ABP_Player_C|GetDirection _asabp_player) 1.8e+02))
                    (Animation|Montage|PlayMontage _mesh "/Game/MW/Player/Animation/Montage/Roll_Montage.Roll_Montage" 1.0 0.0 "Roll_BR"
                      (:then
                        (goto _label_2)))
                    (elif (and (< (Variables|/Game/MW/Player/Blueprints/ABP_Player.ABP_Player_C|GetDirection _asabp_player) 135.0) (>= (Variables|/Game/MW/Player/Blueprints/ABP_Player.ABP_Player_C|GetDirection _asabp_player) 75.0))
                      (Animation|Montage|PlayMontage _mesh "/Game/MW/Player/Animation/Montage/Roll_Montage.Roll_Montage" 1.0 0.0 "Roll_R"
                        (:then
                          (goto _label_2)))
                      (elif (and (>= (Variables|/Game/MW/Player/Blueprints/ABP_Player.ABP_Player_C|GetDirection _asabp_player) -135.0) (< (Variables|/Game/MW/Player/Blueprints/ABP_Player.ABP_Player_C|GetDirection _asabp_player) -75.0))
                        (Animation|Montage|PlayMontage _mesh "/Game/MW/Player/Animation/Montage/Roll_Montage.Roll_Montage" 1.0 0.0 "Roll_L"
                          (:then
                            (goto _label_2)))
                        (elif (and (>= (Variables|/Game/MW/Player/Blueprints/ABP_Player.ABP_Player_C|GetDirection _asabp_player) -75.0) (< (Variables|/Game/MW/Player/Blueprints/ABP_Player.ABP_Player_C|GetDirection _asabp_player) 75.0))
                          (Animation|Montage|PlayMontage _mesh "/Game/MW/Player/Animation/Montage/Roll_Montage.Roll_Montage" 1.0 0.0 "Roll_F"
                            (:then
                              (goto _label_2)))))))))))))
      (else
        (goto _label)))))

(event Input|EnhancedActionEvents|EnhancedInputActionIA_Guard
  (params (ActionValue :type Boolean) (ElapsedSeconds :type Float%20%28double-precision%29) (TriggeredSeconds :type Float%20%28double-precision%29) (InputAction :type Input%20Action%20Object%20Reference :default "/Game/MW/Player/Inputs/IA_Guard.IA_Guard"))
  (bind _shield_collision (Variables|Default|GetShield%20Collision))
  ;[0.15 0.15 0.15 0.5] Guard
  (:Triggered
    (if (> (Variables|Default|GetStamina) 0.0)
      (Variables|Default|SetIsGuarding true)
      (Collision|SetCollisionEnabled _shield_collision "QueryAndPhysics")
      (else
        (Variables|Default|SetIsGuarding false :!label _label)
        (Utilities|FlowControl|Sequence
          (:then_0
            (Collision|SetCollisionEnabled _shield_collision "NoCollision")
            (Variables|Default|SetGuardType -1))
          (:then_1
            (Variables|Default|SetRecoveryingStamina 4e+01)
            (Utilities|FlowControl|Delay 1.0)
            (Variables|Default|SetStaminaRecovery 1))))))
  (:Started
    (Variables|Default|SetStaminaRecovery 0)
    (Variables|Default|SetGuardType 0))
  (:Completed
    (goto _label)))

(event Input|EnhancedActionEvents|EnhancedInputActionIA_Potion
  (params (ActionValue :type Boolean) (ElapsedSeconds :type Float%20%28double-precision%29) (TriggeredSeconds :type Float%20%28double-precision%29) (InputAction :type Input%20Action%20Object%20Reference :default "/Game/MW/Player/Inputs/IA_Potion.IA_Potion"))
  ;[0.15 0.15 0.15 0.5] 포션 마시기
  (:Started
    (if (Math|Boolean|ANDBoolean (> (Variables|Default|GetPotionCount) 0) (not (Variables|Default|GetIsRolling)) (not (Variables|Default|GetIsAttacking)) (not (Variables|Default|GetIsHit)))
      (Variables|Default|SetIsGuarding false)
      (Variables|Default|SetIsDrinking true)
      (Animation|Montage|PlayMontage (Variables|Character|GetMesh) "/Game/MW/Player/Animation/Montage/Potion_Montage.Potion_Montage"
        (:OnInterrupted
          (Variables|Default|SetIsDrinking false))))))

(event Input|EnhancedActionEvents|EnhancedInputActionIA_Attack
  (params (ActionValue :type Boolean) (ElapsedSeconds :type Float%20%28double-precision%29) (TriggeredSeconds :type Float%20%28double-precision%29) (InputAction :type Input%20Action%20Object%20Reference :default "/Game/MW/Player/Inputs/IA_Attack.IA_Attack"))
  (bind _mesh (Variables|Character|GetMesh))
  ;[0.15 0.15 0.15 0.5] Attack
  (:Started
    (if (and (> (Variables|Default|GetStamina) 0.0) (not (Variables|Default|GetIsRolling)))
      (Variables|Default|SetStaminaRecovery 0)
      (if (Variables|Default|GetIsAttacking)
        (Variables|Default|SetIsChainAttacking true)
        (else
          (Variables|Default|SetIsAttacking true)
          (switch int (Variables|Default|GetComboCount) ; 콤보에 따른 분기
            (:0
              (Variables|Default|SetPlayerDamage 50)
              (Animation|Montage|PlayMontage _mesh "/Game/MW/Player/Animation/Montage/Attack_Montage.Attack_Montage" 1.0 0.0 "attack1" false
                (:then
                  (Variables|Default|SetComboCount 1)
                  (bind _output_get (Variables|Default|SetStamina (- (Variables|Default|GetStamina) 3e+01) :!label _label))
                  (if (<= _output_get 0.0)
                    (Variables|Default|SetStamina 0.0)))
                (:OnInterrupted
                  (Variables|Default|SetIsAttacking false :!label _label_2))))
            (:1
              (Variables|Default|SetPlayerDamage 50)
              (Animation|Montage|PlayMontage _mesh "/Game/MW/Player/Animation/Montage/Attack_Montage.Attack_Montage" 1.0 0.0 "attack2" false
                (:then
                  (Variables|Default|SetComboCount 0)
                  (goto _label))
                (:OnInterrupted
                  (goto _label_2))))))))))

(event Input|EnhancedActionEvents|EnhancedInputActionIA_Parry
  (params (ActionValue :type Boolean) (ElapsedSeconds :type Float%20%28double-precision%29) (TriggeredSeconds :type Float%20%28double-precision%29) (InputAction :type Input%20Action%20Object%20Reference :default "/Game/MW/Player/Inputs/IA_Parry.IA_Parry"))
  (:Started
    (if (Math|Boolean|ANDBoolean (not (Variables|Default|GetIsRolling)) (not (Variables|Default|GetIsGettingUp)) (not (Variables|Default|GetIsAttacking)) (not (Variables|Default|GetIsChainAttacking)) (not (Variables|Default|GetIsGuarding)) (not (Variables|Default|GetIsRolling)))
      (Variables|Default|SetStaminaRecovery 0)
      (Variables|Default|SetGuardType 1)
      (Animation|PlayAnimMontage "/Game/MW/Player/Animation/Montage/Player_Parry_Montage.Player_Parry_Montage" 1.0 "None")
      (Variables|Default|SetIsParrying true))))

(event Input|EnhancedActionEvents|EnhancedInputActionIA_Move
  (params (ActionValue :type Vector%202D%20Structure) (ElapsedSeconds :type Float%20%28double-precision%29) (TriggeredSeconds :type Float%20%28double-precision%29) (InputAction :type Input%20Action%20Object%20Reference :default "/Game/MW/Player/Inputs/IA_Move.IA_Move"))
  (bind _returnvalue (Pawn|GetControlRotation :!class /Script/Engine.Pawn))
  ;[0.15 0.15 0.15 0.5] Player Move
  (if (Math|Boolean|NORBoolean (Variables|Default|GetIsRolling) (Variables|Default|GetIsAttacking))
    (Pawn|Input|AddMovementInput (Math|Vector|GetRightVector (Math|Rotator|MakeRotator (.roll _returnvalue) 0.0 (.yaw _returnvalue))) (.y ActionValue) false)
    (Pawn|Input|AddMovementInput (Math|Vector|GetForwardVector (Math|Rotator|MakeRotator 0.0 0.0 (.yaw (Pawn|GetControlRotation :!class /Script/Engine.Pawn)))) (.x ActionValue) false)))

(event Input|EnhancedActionEvents|EnhancedInputActionIA_Camera
  (params (ActionValue :type Vector%202D%20Structure) (ElapsedSeconds :type Float%20%28double-precision%29) (TriggeredSeconds :type Float%20%28double-precision%29) (InputAction :type Input%20Action%20Object%20Reference :default "/Game/MW/Player/Inputs/IA_Camera.IA_Camera"))
  ;[0.15 0.15 0.15 0.5] Camera
  ;;[0.15 0.15 0.15 0.5] L/R
  (Pawn|Input|AddControllerYawInput (.x ActionValue))
  ;;[0.15 0.15 0.15 0.5] U/D
  (Pawn|Input|AddControllerPitchInput (* (.y ActionValue) -1.0)))

(event EventBeginPlay
  ;[0.15 0.15 0.15 0.5] Key mapping
  (Input|AddMappingContext (PlayerController|LocalPlayerSubsystems|GetEnhancedInputLocalPlayerSubsystem (Game|GetPlayerController 0)) "/Game/MW/Player/Inputs/IMC_PlayerInput.IMC_PlayerInput" 0 "(bIgnoreAllPressedKeysUntilRelease=True,bForceImmediately=False,bNotifyUserSettings=False)")
  (Variables|/Script/Engine.CharacterMovementComponent|SetMaxWalkSpeed (Variables|Character|GetCharacterMovement) (Variables|Default|GetWalkSpeed)))

(event Collision|EventActorBeginOverlap
  (params (OtherActor :type Actor%20Object%20Reference)))

(event EventTick
  (params (DeltaSeconds :type Float%20%28single-precision%29))
  ;[0.15 0.15 0.15 0.5] HP/Stamina Rendering
  (Utilities|FlowControl|Sequence
    (:then_0
      (Rendering|Components|TextRender|SetText (Variables|Default|GetHpTextRenderer) (Utilities|Text|ToText(Float) (Variables|Default|GetHp) "HalfToEven"))
      (Rendering|Components|TextRender|SetText (Variables|Default|GetStaminaTextRenderer) (Utilities|Text|ToText(Integer) (Math|Float|Truncate (Variables|Default|GetStamina))))
      (Rendering|Components|TextRender|SetText (Variables|Default|GetTextRender) (Utilities|Text|ToText(Integer) (Variables|Default|GetStaminaRecovery)))
      (Rendering|Components|TextRender|SetText (Variables|Default|Getpotion) (Utilities|Text|ToText(Integer) (Variables|Default|GetGuardType))))
    (:then_1
      (CallFunction|StaminaState (Variables|Default|GetDrowningStamina) (Variables|Default|GetRecoveryingStamina))
      (CallFunction|SetSpeed)
      (CallFunction|HpRecover))))

(fn ConstructionScript)

(fn StaminaState
  (params (DrowningStamina :type Float%20%28double-precision%29) (RecoveryingStamina :type Float%20%28double-precision%29))
  (bind _returnvalue (Utilities|Time|GetWorldDeltaSeconds))
  ;[0.15 0.15 0.15 0.5] -1 : 스테미나 감소
  ; 1 : 스테미나 회복
  (switch int (Variables|Default|GetStaminaRecovery)
    (:-1
      (bind _output_get (Variables|Default|SetStamina (- (Variables|Default|GetStamina) (* DrowningStamina _returnvalue))))
      (if (< _output_get 0.0)
        (Variables|Default|SetStamina 0.0)))
    (:1
      (bind _output_get_2 (Variables|Default|SetStamina (+ (* RecoveryingStamina _returnvalue) (Variables|Default|GetStamina))))
      (if (> _output_get_2 (Variables|Default|GetMaxStamina))
        (Variables|Default|SetStamina (Variables|Default|GetMaxStamina))))))

(fn RollAnimSelectbyDirection
  (bind _asabp_player (Utilities|Casting|CastToABP_Player (Components|SkeletalMesh|GetAnimInstance (Variables|Character|GetMesh))))
  (if (and (>= (Variables|/Game/MW/Player/Blueprints/ABP_Player.ABP_Player_C|GetDirection _asabp_player) -1.8e+02) (< (Variables|/Game/MW/Player/Blueprints/ABP_Player.ABP_Player_C|GetDirection _asabp_player) -135.0))
    (Animation|PlayAnimMontage "/Game/MW/Player/Animation/Montage/Roll_Montage.Roll_Montage" 1.0 "Roll_BL")
    (elif (and (> (Variables|/Game/MW/Player/Blueprints/ABP_Player.ABP_Player_C|GetDirection _asabp_player) 135.0) (<= (Variables|/Game/MW/Player/Blueprints/ABP_Player.ABP_Player_C|GetDirection _asabp_player) 1.8e+02))
      (Animation|PlayAnimMontage "/Game/MW/Player/Animation/Montage/Roll_Montage.Roll_Montage" 1.0 "Roll_BR")
      (elif (and (< (Variables|/Game/MW/Player/Blueprints/ABP_Player.ABP_Player_C|GetDirection _asabp_player) 135.0) (>= (Variables|/Game/MW/Player/Blueprints/ABP_Player.ABP_Player_C|GetDirection _asabp_player) 75.0))
        (Animation|PlayAnimMontage "/Game/MW/Player/Animation/Montage/Roll_Montage.Roll_Montage" 1.0 "Roll_R")
        (elif (and (>= (Variables|/Game/MW/Player/Blueprints/ABP_Player.ABP_Player_C|GetDirection _asabp_player) -135.0) (< (Variables|/Game/MW/Player/Blueprints/ABP_Player.ABP_Player_C|GetDirection _asabp_player) -75.0))
          (Animation|PlayAnimMontage "/Game/MW/Player/Animation/Montage/Roll_Montage.Roll_Montage" 1.0 "Roll_L")
          (elif (and (>= (Variables|/Game/MW/Player/Blueprints/ABP_Player.ABP_Player_C|GetDirection _asabp_player) -75.0) (< (Variables|/Game/MW/Player/Blueprints/ABP_Player.ABP_Player_C|GetDirection _asabp_player) 75.0))
            (Animation|PlayAnimMontage "/Game/MW/Player/Animation/Montage/Roll_Montage.Roll_Montage" 1.0 "Roll_F")))))))

(fn SetSpeed
  (bind _returnvalue (Utilities|Time|GetWorldDeltaSeconds))
  (bind _charactermovement (Variables|Character|GetCharacterMovement))
  (if (Variables|Default|GetIsRunning)
    (Variables|/Script/Engine.CharacterMovementComponent|SetMaxWalkSpeed _charactermovement (Math|Interpolation|FInterpTo (Variables|/Script/Engine.CharacterMovementComponent|GetMaxWalkSpeed _charactermovement) (Variables|Default|GetRunSpeed) _returnvalue 1e+01))
    (elif (Variables|Default|GetIsGuarding)
      (Variables|/Script/Engine.CharacterMovementComponent|SetMaxWalkSpeed _charactermovement (Math|Interpolation|FInterpTo (Variables|/Script/Engine.CharacterMovementComponent|GetMaxWalkSpeed _charactermovement) (Variables|Default|GetGuardingSpeed) _returnvalue 1e+01))
      (else
        (Variables|/Script/Engine.CharacterMovementComponent|SetMaxWalkSpeed _charactermovement (Math|Interpolation|FInterpTo (Variables|/Script/Engine.CharacterMovementComponent|GetMaxWalkSpeed _charactermovement) (Variables|Default|GetWalkSpeed) _returnvalue 1e+01))))))

(fn HpRecover
  (bind _maxhp (LocalVariables|GetMaxHp))
  (if (Variables|Default|GetIsDrinking)
    (LocalVariables|SetCurrentHp (Variables|Default|GetHp))
    (bind _output_get (Variables|Default|SetHpToRecover (+ (Variables|Default|GetPotionRecovery) (Variables|Default|GetHp))))
    (if (> _output_get _maxhp)
      (bind _output_get_2 (Variables|Default|SetHpToRecover _maxhp)))
    (if (> _output_get_2 (LocalVariables|GetCurrentHp))
      (if (Variables|Default|GetIsHit)
        (Variables|Default|SetHp (LocalVariables|GetCurrentHp))
        (return)
        (else
          (bind _output_get_3 (Variables|Default|SetHp (+ (LocalVariables|GetCurrentHp) (* (Utilities|Time|GetWorldDeltaSeconds) 20.814))))
          (if (>= _output_get_3 (Variables|Default|GetHpToRecover))
            (Variables|Default|SetHp (Variables|Default|GetHpToRecover))
            (return)))))))

(fn CancelStatus
  (Variables|Default|SetIsDrinking false)
  (Variables|Default|SetIsAttacking false)
  (Variables|Default|SetIsRunning false)
  (Variables|Default|SetIsChainAttacking false))