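; Game mode that drives HUD and audio for a fight against BP_Knight, from start to win/lose screen.
; BeginPlay shows player UI; external events toggle a draw-weapon prompt, and WeaponOut refills the knight's HP and displays its health UI.
; WhenFinished, guarded by DeadFlag, swaps enemy UI for animated result text and sound, removing it after a delay on loss.
; ManageBGM uses a FlipFlop to alternately create and stop music.
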(event Custom|ManageBGM
  ;[0.15 0.15 0.15 0.5] BGM OnOff
  (Utilities|FlowControl|FlipFlop
    (:A
      (bind _returnvalue (AddComponent|AddAudioComponent false))
      (Variables|Default|SetBGM _returnvalue))
    (:B
      (Audio|Components|Audio|Stop (Variables|Default|GetBGM)))))

(event Custom|Display_WeaponOut
  ;[0.15 0.15 0.15 0.5] 무기 뽑으라는 UI 뜸
  (bind _returnvalue (UserInterface|CreateWidget "/Game/YW/UI/WBP_WeaponOut.WBP_WeaponOut_C"))
  (UserInterface|Viewport|AddtoViewport _returnvalue 0)
  (Variables|Default|SetWithin_UI_Distance true))

(event Custom|Remove_Display_WeaponOut
  ;[0.15 0.15 0.15 0.5] 무기를 뽑으면 UI 사라짐
  (Widget|RemovefromParent (stale Custom|Display_WeaponOut _returnvalue))
  (Variables|Default|SetWithin_UI_Distance false)
  (Variables|Default|SetWithin_WeaponOut_Distance false))

(event Custom|WhenFinished
  ;[0.15 0.15 0.15 0.5] 게임 오버
  (if (== (Variables|Default|GetDeadFlag) false)
    (Variables|Default|SetDeadFlag true)
    (Widget|RemovefromParent (stale Custom|WeaponOut _returnvalue_2))
    (bind _returnvalue (UserInterface|CreateWidget "/Game/YW/UI/WBP_Lose_Or_Win.WBP_Lose_Or_Win_C"))
    (UserInterface|Viewport|AddtoViewport _returnvalue 0)
    (CallFunction|ManageBGM)
    (if (Math|Conversions|ToBoolean(Integer) (Variables|Default|GetPlayerLose))
      (Default|LoseTextAnim _returnvalue)
      (Audio|PlaySound2D "/Game/Sounds/You_Died.You_Died" 1.0 1.0 0.0 0 0)
      (Utilities|FlowControl|Delay 3.0)
      (CallFunction|RemoveFinishUI)
      (else
        (Default|WinTextAnim _returnvalue)
        (Audio|PlaySound2D "/Game/Sounds/Heir.Heir" 1.0 1.0 0.0 0 0)))))

(event Custom|WeaponOut
  ;[0.15 0.15 0.15 0.5] 무기 뽑으면 Enemy HP 뜸
  (bind _returnvalue (Actor|GetActorOfClass "/Game/YW/blueprint/BP_Knight.BP_Knight_C"))
  (Variables|/Game/YW/blueprint/BP_Knight.BP_Knight_C|SetHP _returnvalue (Variables|/Game/YW/blueprint/BP_Knight.BP_Knight_C|GetMaxHP _returnvalue))
  (bind _returnvalue_2 (UserInterface|CreateWidget "/Game/YW/UI/WBP_Enemy_UI.WBP_Enemy_UI_C"))
  (UserInterface|Viewport|AddtoViewport _returnvalue_2 0)
  (bind _returnvalue_3 (Actor|GetActorOfClass "/Game/YW/blueprint/BP_Knight.BP_Knight_C"))
  (Variables|/Game/YW/UI/WBP_Enemy_UI.WBP_Enemy_UI_C|SetEnemyActor _returnvalue_2 _returnvalue_3))

(event Custom|RemoveFinishUI
  ;[0.15 0.15 0.15 0.5] 게임 오버
  (Widget|RemovefromParent (stale Custom|WhenFinished _returnvalue)))

(event EventBeginPlay
  ;[0.15 0.15 0.15 0.5] 시작 : 플레이어 HP 뜸
  (Variables|Default|SetDeadFlag false)
  (bind _returnvalue (UserInterface|CreateWidget "/Game/YW/UI/WBP_Player_UI.WBP_Player_UI_C"))
  (UserInterface|Viewport|AddtoViewport _returnvalue 0)
  (Variables|Default|SetWithin_UI_Distance false)
  (Audio|PlaySound2D "/Game/Sounds/Retrieval.Retrieval" 1.0 1.0 0.0 0 0))

(event EventTick
  (params (DeltaSeconds :type Float%20%28single-precision%29)))

(fn ConstructionScript)