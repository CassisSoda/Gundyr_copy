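; Lock-on component for BP_Player that toggles targeting of a pawn with the IA_LockOn input.
; On press it clears the current target, or sphere-traces forward from just above the camera for a pawn, with debug drawing enabled.
; Locking switches character movement from orient-to-movement to controller-desired rotation and sets IsLockOn; unlocking reverts both.
; Tick points the control rotation at the target with a slight downward pitch offset.
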(event Input|EnhancedActionEvents|EnhancedInputActionIA_LockOn
  (params (ActionValue :type Boolean) (ElapsedSeconds :type Float%20%28double-precision%29) (TriggeredSeconds :type Float%20%28double-precision%29) (InputAction :type Input%20Action%20Object%20Reference :default "/Game/MW/Player/Inputs/IA_LockOn.IA_LockOn"))
  (bind _returnvalue (Game|GetPlayerCameraManager 0))
  (bind _playerbp (Variables|Default|GetPlayerBP))
  (bind _playerbp_2 (Variables|Default|GetPlayerBP))
  (bind _transformcomponent (Variables|/Script/Engine.PlayerCameraManager|GetTransformComponent _returnvalue))
  (bind _charactermovement (Variables|/Script/Engine.Character|GetCharacterMovement _playerbp_2))
  (bind _charactermovement_2 (Variables|/Script/Engine.Character|GetCharacterMovement _playerbp))
  (bind _returnvalue_2 (Transformation|GetWorldLocation _transformcomponent))
  (bind _returnvalue_3 (+ (.z _returnvalue_2) 3e+01))
  (bind _returnvalue_4 (Math|Vector|MakeVector (.x _returnvalue_2) (.y _returnvalue_2) _returnvalue_3))
  ;[0.15 0.15 0.15 0.5] Lock on 기능
  (:Started
    (Variables|Default|GetTargetLockActor
      (:then
        (Variables|Default|SetTargetLockActor 0)
        (Variables|/Script/Engine.CharacterMovementComponent|SetbOrientRotationToMovement _charactermovement_2 true)
        (Variables|/Script/Engine.CharacterMovementComponent|SetbUseControllerDesiredRotation _charactermovement_2 false)
        (Variables|/Game/MW/Player/Blueprints/BP_Player.BP_Player_C|SetIsLockOn _playerbp false))
      (:else
        (bind (_outhit _returnvalue_5) (Collision|SphereTraceForObjects _returnvalue_4 (+ _returnvalue_4 (* (Math|Vector|GetForwardVector (Transformation|GetWorldRotation _transformcomponent)) 1e+03)) 2e+02 (Utilities|Array|MakeArray "ObjectTypeQuery3") false 0 "ForDuration" true "(R=1.000000,G=0.000000,B=0.000000,A=1.000000)" "(R=0.000000,G=1.000000,B=0.000000,A=1.000000)" 2.0))
        (if _returnvalue_5
          (Variables|Default|SetTargetLockActor (.HitActor (Collision|BreakHitResult _outhit)))
          (Variables|/Script/Engine.CharacterMovementComponent|SetbOrientRotationToMovement _charactermovement false)
          (Variables|/Script/Engine.CharacterMovementComponent|SetbUseControllerDesiredRotation _charactermovement true)
          (Variables|/Game/MW/Player/Blueprints/BP_Player.BP_Player_C|SetIsLockOn _playerbp_2 true))))))

(event EventTick
  (params (DeltaSeconds :type Float%20%28single-precision%29))
  (bind _targetlockactor (Variables|Default|GetTargetLockActor))
  (bind _playerbp (Variables|Default|GetPlayerBP))
  (bind _returnvalue (Transformation|GetActorLocation _playerbp))
  (bind _returnvalue_2 (Transformation|GetActorLocation _targetlockactor))
  (bind _returnvalue_3 (Math|Rotator|FindLookatRotation _returnvalue _returnvalue_2))
  ;[0.15 0.15 0.15 0.5] Target Lock update
  (Variables|Default|GetTargetLockActor
    (:then
      (Pawn|SetControlRotation (Pawn|GetController (Variables|Default|GetPlayerBP)) (Math|Rotator|MakeRotator (.roll _returnvalue_3) (- (.pitch _returnvalue_3) 5.0) (.yaw _returnvalue_3))))
    (:else)))

(event EventBeginPlay
  ;[0.15 0.15 0.15 0.5] Get Player
  (bind _asbp_player (Utilities|Casting|CastToBP_Player (Components|GetOwner)))
  (Variables|Default|SetPlayerBP _asbp_player))